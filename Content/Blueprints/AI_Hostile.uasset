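; AI_Hostile is a hostile AI character that fires projectiles and carries a colour.
; Each tick it sets its walk speed from SpeedRate multiplied by SpeedVariable.
; AiAttack spawns a Projectile at the actor's transform and initialises it with the current colour, a fixed size, itself as attach target and an attacker type.
; SetColour stores the colour that later shots pass on.
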(event `self.ReceiveTick`
  (params (DeltaSeconds :type "Float (single-precision)"))
  (set `CharacterMovementComponent.MaxWalkSpeed` (* (`self.speedRate`) (`self.speedVariable`)) (`self.CharacterMovement`)))

(fn `aiAttack`
  (bind _returnvalue (`|SpawnActorFromClass` "/Game/Blueprints/Projectile.Projectile_C" (`self.GetTransform` self) "Undefined" "OverrideRootScale" self))
  (bind _asprojectile (cast `/Game/Blueprints/Projectile` _returnvalue))
  (`/Game/Blueprints/Projectile.instantiate` _asprojectile (`self.Colour`) 30.0 self 2))

(fn `setColour`
  (params (colourIn :type Integer))
  (set `self.Colour` colourIn))

(fn `UserConstructionScript`)