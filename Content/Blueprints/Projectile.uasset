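; Colour-coded attack Projectile that attaches to a target actor and grows as an expanding sphere.
; Instantiate sets colour, maximum size and attacker type, then Tick applies the matching material and lerps the scale until it reaches maximum and destroys itself.
; On overlap, attacker type 1 destroys hostile AI of the same colour, while any other type damages the top-down player character regardless of colour.
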(event `self.ReceiveTick`
  (params (DeltaSeconds :type "Float (single-precision)"))
  (bind _colour (`self.Colour`))
  (if (!= (`self.Colour`) 0)
    (if (== _colour 1)
      (`PrimitiveComponent.SetMaterial` (`self.Sphere`) 0 "/Game/Blueprints/Blue.Blue")
      (elif (== _colour 2)
        (`PrimitiveComponent.SetMaterial` (`self.Sphere`) 0 "/Game/Blueprints/Red.Red")
        (elif (<= _colour 3)
          (`PrimitiveComponent.SetMaterial` (`self.Sphere`) 0 "/Game/Blueprints/Green.Green")
          (else
            (`PrimitiveComponent.SetMaterial` (`self.Sphere`) 0 "/Game/Blueprints/Yellow.Yellow")))))
    (if (>= (`KismetMathLibrary.VSize` (`self.GetActorScale3D`)) (`KismetMathLibrary.VSize` (`self.MaxSize`)))
      (`self.K2_DestroyActor`)
      (else
        (bind _output_get (set `self.Counter` (+ (* DeltaSeconds 2.0) (`self.Counter`))))
        (`self.SetActorScale3D` (`KismetMathLibrary.VLerp` (`self.OriginalScale`) (`self.MaxSize`) _output_get))))))

(event `self.ReceiveActorBeginOverlap`
  (params (OtherActor :type "Actor Object Reference"))
  (if (== (`self.attackerType`) 1)
    (bind _outactors (`GameplayStatics.GetAllActorsOfClass` "/Game/Blueprints/AI_Hostile.AI_Hostile_C"))
    (for _array_element _outactors
      (if (== OtherActor _array_element)
        (if (== (`self.Colour`) (`/Game/Blueprints/AI_Hostile.Colour` _array_element))
          (`self.K2_DestroyActor` _array_element))))
    (else
      (bind _outactors_2 (`GameplayStatics.GetAllActorsOfClass` "/Game/Blueprints/TopDownCharacter.TopDownCharacter_C"))
      (for _array_element_2 _outactors_2
        (if (== OtherActor _array_element_2)
          (`/Game/Blueprints/TopDownCharacter.damagePlayer` _array_element_2))))))

(fn `instantiate`
  (params (ColourIn :type Integer) (SizeIn :type "Float (double-precision)") (targetToAttach :type "Actor Object Reference") (attackerType :type Integer))
  (`self.K2_AttachToActor` targetToAttach "None" "SnapToTarget" "KeepRelative" "KeepRelative")
  (bind _output_get (set `self.MaxSize` (`KismetMathLibrary.MakeVector` SizeIn SizeIn SizeIn)))
  (set `self.Colour` ColourIn)
  (set `self.MaxSize` _output_get)
  (set `self.attackerType` attackerType))

(fn `UserConstructionScript`)